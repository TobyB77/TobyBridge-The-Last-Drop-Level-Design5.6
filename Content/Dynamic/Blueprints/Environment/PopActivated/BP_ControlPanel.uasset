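; Control panel environment prop that triggers an activatable and visibly sparks when it receives a Pop interaction.
; On interaction it calls ActivateDeactivate on BPActivatable, then waits briefly before spawning Niagara sparks at its Billboard, swapping a mesh material slot to BaseFlattenMaterial and playing a 2D sound.
; The construction script only calls the parent's.
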(event EventBPIPopInteract
  (Default|Activate/Deactivate (Variables|Default|GetBP_Activatable))
  (Utilities|FlowControl|Delay 0.3)
  (Niagara|SpawnSystematLocation "/Game/Dynamic/Blueprints/Environment/NS_Sparks.NS_Sparks" (Transformation|GetWorldLocation (Variables|Default|GetBillboard)))
  (Rendering|Material|SetMaterial (Variables|Default|GetStaticMesh) 1 "/Engine/EngineMaterials/BaseFlattenMaterial.BaseFlattenMaterial")
  (Audio|PlaySound2D "/Game/Dynamic/Audio/Events/MS_ControlPanel.MS_ControlPanel" 1.0 1.0 0.0 0 0))

(fn ConstructionScript
  (|CallParentFunction))